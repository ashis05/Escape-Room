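; BP_TV is a television actor that shows a start widget and plays a video on a plane.
; On BeginPlay it hands itself to its W_PlayVideo widget and pre-opens a fixed media source on the 2DVideo player, with autoplay and looping disabled.
; The StartVideo event, exposed through that reference, hides the widget component, plays the player and reveals the Plane.
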(event Custom|StartVideo
  (Rendering|SetVisibility (Variables|Default|GetWidget) false false)
  (Media|MediaPlayer|Play (Variables|Default|Get2DVideo) :!class /Script/MediaAssets.MediaPlayer)
  (Rendering|SetVisibility (Variables|Default|GetPlane) true false))

(event EventBeginPlay
  (bind _asw_play_video (Utilities|Casting|CastToW_PlayVideo (UserInterface|GetUserWidgetObject (Variables|Default|GetWidget))))
  (Variables|/Game/Television/W_PlayVideo.W_PlayVideo_C|SetBP_TV _asw_play_video self)
  (Class|MediaPlayer|OpenSourceLatent (Variables|Default|Get2DVideo) "/Game/Television/VID-20210812-WA0011.VID-20210812-WA0011" (Utilities|Struct|MakeMediaPlayerOptions "(Audio=0,Caption=-1,Metadata=-1,Script=-1,Subtitle=-1,Text=-1,Video=0)" "+00000000.00:00:00.000000000" "Disabled" "Disabled")))

(event Collision|EventActorBeginOverlap
  (params (OtherActor :type Actor%20Object%20Reference)))

(event EventTick
  (params (DeltaSeconds :type Float%20%28single-precision%29)))

(fn ConstructionScript)